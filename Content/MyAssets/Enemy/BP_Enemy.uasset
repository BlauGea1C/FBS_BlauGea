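; BP_Enemy is an enemy pawn that runs one of three idle movement behaviours (Patrol, Roam or Guard), chosen by BaseBehaviour on BeginPlay.
; Patrol follows linked patrol points with random pauses on arrival.
; Roam re-targets random navigable locations around its PatrolPoint on a random timer started at move request, rerolling nearby picks.
; Guard moves to its PatrolPoint, then uses a timeline to rotate to that point's facing.
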(event `self.ReceiveBeginPlay`
  (`self.LaunchBaseBehaviour`))

(event `LaunchBaseBehaviour`
  (switch `/Game/MyAssets/Enum_EnemyStates` (`self.BaseBehaviour`)
    (:`NewEnumerator0`
      (`self.BehaviourPatrol`))
    (:`NewEnumerator1`
      (`self.BehaviourRoam`))
    (:`NewEnumerator2`
      (`self.BehaviorGuard`))))

(event `BehaviorGuard`
  (`|AIMoveTo` self (0.0 0.0 0.0) (`self.PatrolPoint`) 1.0
    (:`OnSuccess`
      (set `self.Guard_InitialRotation` (`self.K2_GetActorRotation`))
      (set `self.Guard_EndRotation` (`self.K2_GetActorRotation` (`self.PatrolPoint`)))
      (bind (_direction _alpha) (`Timeline|GuardRotationAnimation`)
        (:`Update`
          (`self.K2_SetActorRotation` (`KismetMathLibrary.RLerp` (`self.Guard_InitialRotation`) (`self.Guard_EndRotation`) _alpha true)))))))

(event `BehaviourPatrol`
  (`|AIMoveTo` self (0.0 0.0 0.0) (`self.PatrolPoint`) 50.0
    (:`OnSuccess`
      (`KismetSystemLibrary.Delay` (`KismetMathLibrary.RandomFloatInRange` 2.0 5.0))
      (set `self.PatrolPoint` (`/Game/MyAssets/BP_PatrolPoint.NextPatrolPoit` (`self.PatrolPoint`)))
      (`self.BehaviourPatrol`))))

(event `BehaviourRoam`
  (bind _randomlocation (`NavigationSystemV1.K2_GetRandomLocationInNavigableRadius` (`self.K2_GetActorLocation` (`self.PatrolPoint`)) (`self.RoamRadiuS`) null null))
  (if (> (`KismetMathLibrary.Vector_Distance` _randomlocation (`self.K2_GetActorLocation`)) 200.0)
    (`|AIMoveTo` self _randomlocation null 1.0
      (:`then`
        (`KismetSystemLibrary.Delay` (`KismetMathLibrary.RandomFloatInRange` 2.0 5.0))
        (`self.BehaviourRoam`)))
    (else
      (`self.BehaviourRoam`))))

(fn `UserConstructionScript`)