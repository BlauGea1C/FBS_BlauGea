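; Vel'Koz enemy that patrols, roams or guards a point until it aggros on the player.
; Sight, damage or a Cry event triggers aggro; sight and damage alerts also spawn BP_EnemyAlert.
; It chases via AIMoveTo and fires projectiles, choosing montages by distance, while repeated sightings refresh a retriggerable timer that restores base behaviour.
; A HealthManager macro routes damage to death, which plays a montage and dissolve before destroying the actor.
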(event `self.ReceiveBeginPlay`
  (`self.LaunchBaseBehaviour`)
  (bind _asbp_third_person_character (cast `/Game/ThirdPerson/Blueprints/BP_ThirdPersonCharacter` (`GameplayStatics.GetPlayerCharacter` 0)))
  (set `self.Ashe` _asbp_third_person_character))

(event `LaunchBaseBehaviour`
  (switch `/Game/MyAssets/Enum_EnemyStates` (`self.BaseBehaviour`)
    (:`NewEnumerator0`
      (`self.BehaviourPatrol`))
    (:`NewEnumerator1`
      (`self.BehaviourRoam`))
    (:`NewEnumerator2`
      (`self.BehaviorGuard`))))

(event `BehaviorGuard`
  ; GUARD
  (if (not (`self.HasAggro`))
    (`|AIMoveTo` self (0.0 0.0 0.0) (`self.PatrolPoint`) 1.0
      (:`OnSuccess`
        (set `self.Guard_InitialRotation` (`self.K2_GetActorRotation`))
        (set `self.Guard_EndRotation` (`self.K2_GetActorRotation` (`self.PatrolPoint`)))
        (bind (_direction _alpha) (`Timeline|GuardRotationAnimation`)
          (:`Update`
            (`self.K2_SetActorRotation` (`KismetMathLibrary.RLerp` (`self.Guard_InitialRotation`) (`self.Guard_EndRotation`) _alpha true))))))))

(event `BehaviourPatrol`
  ;[0.002732 0.15 0.000911 0.502] PATROL
  (if (not (`self.HasAggro`))
    (`|AIMoveTo` self (0.0 0.0 0.0) (`self.PatrolPoint`) 50.0
      (:`OnSuccess`
        (`KismetSystemLibrary.Delay` (`KismetMathLibrary.RandomFloatInRange` 2.0 5.0))
        (set `self.PatrolPoint` (`/Game/MyAssets/BP_PatrolPoint.NextPatrolPoit` (`self.PatrolPoint`)))
        (`self.BehaviourPatrol`)))))

(event `BehaviourRoam`
  ;[0.02807 0.02447 0.15 0.5] ROAM
  (if (not (`self.HasAggro`))
    (bind _randomlocation (`NavigationSystemV1.K2_GetRandomLocationInNavigableRadius` (`self.K2_GetActorLocation` (`self.PatrolPoint`)) (`self.RoamRadiuS`) null null))
    (if (> (`KismetMathLibrary.Vector_Distance` _randomlocation (`self.K2_GetActorLocation`)) 200.0)
      (`|AIMoveTo` self _randomlocation null 1.0
        (:`then`
          (`KismetSystemLibrary.Delay` (`KismetMathLibrary.RandomFloatInRange` 2.0 5.0))
          (`self.BehaviourRoam`)))
      (else
        (`self.BehaviourRoam`)))))

(event `self.OnShot`
  (params (DirectionShoot :type "Vector Structure") (Damage :type "Float (double-precision)"))
  ;[0.15 0.06616 0 0.5] Daño Muerte
  (`self.HealthManager` Damage
    (:`IsDead`
      (`self.Dead`))
    (:`IsAlive`
      (if (not (`self.HasAggro`))
        (`/Engine/EditorBlueprintResources/StandardMacros.DoOnce` false
          (:`Completed`
            (`self.BehaviorAlert`)))))))

(event `/Game/MyAssets/BPI_Damageable.OnDamaged`
  (params (NewParam :type "Float (double-precision)"))
  ;[0.15 0.06616 0 0.5] Daño Muerte
  ;; DañoBarril
  (`self.HealthManager` NewParam
    (:`IsDead`
      (`self.Dead`))
    (:`IsAlive`
      (if (not (`self.HasAggro`))
        (`self.BehaviorAlert`)))))

(event `Dead`
  ;[0.15 0.06616 0 0.5] Daño Muerte
  (`/Engine/EditorBlueprintResources/StandardMacros.DoOnce` false
    (:`Completed`
      (`KismetSystemLibrary.PrintString` "VelkozDead")
      (`self.BehaviorStop`)
      (`CharacterMovementComponent.SetMovementMode` (`self.CharacterMovement`) "MOVE_None" 0)
      (bind _returnvalue (`self.PlayAnimMontage` "/Game/MyAssets/Enemys/Enemy_Velkoz/AM_Velkoz_Death.AM_Velkoz_Death"))
      (`ActorComponent.K2_DestroyComponent` (`self.ProjectileVelkoz`))
      (set `PawnSensingComponent.SightRadius` 0.0 (`self.PawnSensing`))
      (`self.BehaviorStop`)
      (bind (_direction _dissolve) (`Timeline|Dissolve` :!via `PlayFromStart`)
        (:`Update`
          (`MeshComponent.SetScalarParameterValueOnMaterials` (`self.Mesh`) "Dissolve" (`KismetMathLibrary.Lerp` -1.0 1.0 _dissolve)))
        (:`Finished`
          (`KismetSystemLibrary.Delay` _returnvalue)
          (`self.K2_DestroyActor`))))))

(event `BehaviorAlert`
  ;[0.15 0.001176 0.0205 0.5] DETECTAR AL JUGADOR * ATACAR
  (`/Engine/EditorBlueprintResources/StandardMacros.DoOnce` false :!label _label
    (:`Completed`
      (set `self.HasAggro` true)
      (`self.BehaviorStop`)
      (`|SpawnActorFromClass` "/Game/MyAssets/BP_EnemyAlert.BP_EnemyAlert_C" (`KismetMathLibrary.MakeTransform` (`self.K2_GetActorLocation`)) "Undefined" "MultiplyWithRoot" null null)
      (bind _returnvalue (`self.PlayAnimMontage` "/Game/MyAssets/Enemys/Enemy_Velkoz/AM_Velkoz_AreaAlert.AM_Velkoz_AreaAlert"))
      (`KismetSystemLibrary.Delay` _returnvalue)
      (if (not (<= (`self.Health`) 0.0))
        (`self.BehaviorChase`)))))

(event `self.PawnSensing.OnSeePawn`
  (params (Pawn :type "Pawn Object Reference"))
  ;[0.15 0.001176 0.0205 0.5] DETECTAR AL JUGADOR * ATACAR
  ;; DETECTOR
  (if (== Pawn (`self.Ashe`))
    (if (not (`self.HasAggro`))
      (`self.BehaviorAlert`)
      (else
        (`self.TryNotSeePawn`)))))

(event `ResetAlert`
  ;[0.15 0.001176 0.0205 0.5] DETECTAR AL JUGADOR * ATACAR
  (goto _label :!via `Reset`))

(event `BehaviorStop`
  ;[0.15 0.001176 0.0205 0.5] DETECTAR AL JUGADOR * ATACAR
  (`|AIMoveTo` self (0.0 0.0 0.0) self))

(event `Cry`
  ;[0.15 0.001176 0.0205 0.5] DETECTAR AL JUGADOR * ATACAR
  ;; ALARMA
  (if (not (`self.HasAggro`))
    (set `self.HasAggro` true)
    (`self.BehaviorStop`)
    (bind _returnvalue (`self.PlayAnimMontage` "/Game/MyAssets/Enemys/Enemy_Velkoz/AM_Velkoz_Cry.AM_Velkoz_Cry"))
    (`KismetSystemLibrary.Delay` _returnvalue)
    (`self.BehaviorChase`)))

(event `BehaviorChase`
  ;[0.15 0.001176 0.0205 0.5] DETECTAR AL JUGADOR * ATACAR
  ;; PERSECUCION
  (`|AIMoveTo` self (0.0 0.0 0.0) (`self.Ashe`) (`self.AttackDistance`)
    (:`OnSuccess`
      (`KismetSystemLibrary.PrintString` "VelkozPersecucion" true true (struct :`R` 0.859375 :`G` 0.042427 :`B` 0.003339 :`A` 1.0))
      (`self.BehaviorAttack`))))

(event `TryNotSeePawn`
  ;[0.15 0.001176 0.0205 0.5] DETECTAR AL JUGADOR * ATACAR
  (`KismetSystemLibrary.RetriggerableDelay` 5.0)
  (`self.BehaviorStop`)
  (set `self.HasAggro` false)
  (`self.ResetAlert`)
  (`KismetSystemLibrary.Delay` 2.0)
  (if (not (`self.HasAggro`))
    (`self.LaunchBaseBehaviour`)))

(event `BehaviorAttack`
  ;[0.15 0.001176 0.0205 0.5] DETECTAR AL JUGADOR * ATACAR
  ;; ATAQUE
  (`/Engine/EditorBlueprintResources/StandardMacros.DoOnce` false :!label _label_2
    (:`Completed`
      (`self.BehaviorStop`)
      (if (<= (`KismetMathLibrary.Vector_Distance` (`self.K2_GetActorLocation`) (`self.K2_GetActorLocation` (`self.Ashe`))) 2000.0)
        ;;; CLOSE
        (`GameplayStatics.PlaySound2D` "/Game/MyAssets/Enemys/Enemys/SC_AttackVelcoz.SC_AttackVelcoz" 1.0 1.0 0.0 null null)
        (bind _returnvalue (`self.PlayAnimMontage` "/Game/MyAssets/Enemys/Enemy_Velkoz/AM_Velkoz_Attack1.AM_Velkoz_Attack1"))
        (`KismetSystemLibrary.PrintString` "ATTACK CLOSE  -velkoz" true true (struct :`R` 0.859375 :`G` 0.042427 :`B` 0.003339 :`A` 1.0))
        (`self.Projectile`)
        (`KismetSystemLibrary.Delay` _returnvalue)
        (else
          ;;; MID
          (`GameplayStatics.PlaySound2D` "/Game/MyAssets/Enemys/Enemys/SC_AttackVelcoz.SC_AttackVelcoz" 1.0 1.0 0.0 null null)
          (bind _returnvalue_2 (`self.PlayAnimMontage` "/Game/MyAssets/Enemys/Enemy_Velkoz/AM_Velkoz_Attack2.AM_Velkoz_Attack2"))
          (`KismetSystemLibrary.PrintString` "ATTACK MID velkoz" true true (struct :`R` 0.859375 :`G` 0.042427 :`B` 0.003339 :`A` 1.0))
          (`self.Projectile`)
          (`KismetSystemLibrary.Delay` _returnvalue_2)))
      (`self.ResetAttack`)
      (`self.BehaviorChase`))))

(event `Projectile`
  ;[0.15 0.001176 0.0205 0.5] DETECTAR AL JUGADOR * ATACAR
  ;; ATAQUE
  (`self.RedirectAttack`)
  (`|SpawnActorFromClass` "/Game/MyAssets/BP_ProjectileVelkoz.BP_ProjectileVelkoz_C" (`KismetMathLibrary.MakeTransform` (`SceneComponent.K2_GetComponentLocation` (`self.ProjectileVelkoz`)) (`KismetMathLibrary.Conv_VectorToRotator` (`SceneComponent.GetForwardVector` (`self.CapsuleComponent`)))) "Undefined" "MultiplyWithRoot" null null))

(event `ResetAttack`
  ;[0.15 0.001176 0.0205 0.5] DETECTAR AL JUGADOR * ATACAR
  ;; ATAQUE
  (goto _label_2 :!via `Reset`))

(event `RedirectAttack`
  ;[0.15 0.001176 0.0205 0.5] DETECTAR AL JUGADOR * ATACAR
  ;; ATAQUE
  (`self.K2_SetActorRotation` (`KismetMathLibrary.FindLookAtRotation` (`self.K2_GetActorLocation`) (`self.K2_GetActorLocation` (`self.Ashe`)))))

(fn `UserConstructionScript`)