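; BP_Weapon is the player's weapon, firing Basic, Special, Ultimate and Flare projectiles from the muzzle along the follow camera's aim.
; Shoot routes each attack type through DoOnce gates, with ammo costs and cooldowns per attack.
; Basic counts shots toward a triple burst, resetting after a pause, while Special spawns an angled fan.
; Reload refills the magazine from the character's ammo reserve after a delay, blocking fire meanwhile.
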(event `self.ReceiveBeginPlay`
  (bind _asbp_third_person_character (cast `/Game/ThirdPerson/Blueprints/BP_ThirdPersonCharacter` (`GameplayStatics.GetPlayerCharacter` 0)))
  (set `self.Ashe` _asbp_third_person_character))

(event `ResetBase`
  (goto _label :!via `Reset`))

(event `/Game/MyAssets/BPI_Weapone.Shoot`
  (params (AttackTipe :type "/Game/MyAssets/Enum_AttackTipe Enum" :default "NewEnumerator0"))
  (if (not (`self.IsReloading`))
    (switch `/Game/MyAssets/Enum_AttackTipe` AttackTipe
      (:`NewEnumerator0`
        (`/Engine/EditorBlueprintResources/StandardMacros.DoOnce` false :!label _label
          (:`Completed`
            (`self.CheckAmmo` (`self.AttackBasic_Cost`)
              (:`OK`
                (`self.Attack_Basic`)
                (`KismetSystemLibrary.Delay` (`self.Attack_Basic_CoolDown`)))
              (:`Denied`
                _))
            (`self.ResetBase`))))
      (:`NewEnumerator1`
        (`/Engine/EditorBlueprintResources/StandardMacros.DoOnce` false :!label _label_2
          (:`Completed`
            (`self.CheckAmmo` (`self.AttackSpecial_Cost`)
              (:`OK`
                (`self.Attack_Special`))
              (:`Denied`
                _))
            (`self.ResetSpecial`))))
      (:`NewEnumerator2`
        (`/Engine/EditorBlueprintResources/StandardMacros.DoOnce` false :!label _label_3
          (:`Completed`
            (`self.CheckAmmo` (`self.AttackUltimate_Cost`)
              (:`OK`
                (`self.Attack_Ultimate`))
              (:`Denied`
                _))
            (`self.ResetUltimate`))))
      (:`NewEnumerator3`
        (`/Engine/EditorBlueprintResources/StandardMacros.DoOnce` false :!label _label_4
          (:`Completed`
            (`self.CheckAmmo` (`self.AttackFlare_Cost`)
              (:`OK`
                (`/Game/MyAssets/BPI_Weapone.Attack_Flare`))
              (:`Denied`
                _))
            (`self.ResetFlare`)))))))

(event `ResetSpecial`
  (`KismetSystemLibrary.Delay` (`self.Attack_Special_CoolDown`))
  (goto _label_2 :!via `Reset`))

(event `ResetUltimate`
  (`KismetSystemLibrary.Delay` (`self.Attack_Ultimate_CoolDown`))
  (goto _label_3 :!via `Reset`))

(event `ResetFlare`
  (`KismetSystemLibrary.Delay` (`self.Attack_Flare_CoolDown`))
  (goto _label_4 :!via `Reset`))

(event `ProjectileFlare`
  ; SPAWN DE PROYECTILES ROTACION Y DIRECCION Flare
  (`|SpawnActorFromClass` "/Game/MyAssets/BP_Projectile_Flare.BP_Projectile_Flare_C" (`KismetMathLibrary.MakeTransform` (`SceneComponent.K2_GetComponentLocation` (`self.Muzzle`)) (`KismetMathLibrary.Conv_VectorToRotator` (`SceneComponent.GetForwardVector` (`/Game/ThirdPerson/Blueprints/BP_ThirdPersonCharacter.FollowCamera` (`self.Ashe`))))) "Undefined" "MultiplyWithRoot" null null))

(event `ProjectileBasic`
  ; SPAWN DE PROYECTILES ROTACION Y DIRECCION basic
  (`|SpawnActorFromClass` "/Game/MyAssets/BP_Projectile.BP_Projectile_C" (`KismetMathLibrary.MakeTransform` (`SceneComponent.K2_GetComponentLocation` (`self.Muzzle`)) (`KismetMathLibrary.Conv_VectorToRotator` (`SceneComponent.GetForwardVector` (`/Game/ThirdPerson/Blueprints/BP_ThirdPersonCharacter.FollowCamera` (`self.Ashe`))))) "Undefined" "MultiplyWithRoot" null null))

(event `/Game/MyAssets/BPI_Weapone.Attack_Flare`
  (`KismetSystemLibrary.PrintString` "FLARE")
  (`self.ProjectileFlare`))

(event `/Game/MyAssets/BPI_Weapone.Attack_Basic`
  (`KismetSystemLibrary.PrintString` "BASIC")
  (if (< (`self.AttackBasic_Count`) 3)
    (`self.ProjectileBasic`)
    (`/Engine/EditorBlueprintResources/StandardMacros.IncrementInt` (`self.AttackBasic_Count`)
      (:`  `
        (`KismetSystemLibrary.RetriggerableDelay` 2.0)
        (set `self.AttackBasic_Count` 0)))
    (else
      (`self.ProjectileBasic`)
      (`KismetSystemLibrary.Delay` 0.2)
      (`self.ProjectileBasic`)
      (`KismetSystemLibrary.Delay` 0.2)
      (`self.ProjectileBasic`)
      (set `self.AttackBasic_Count` 0))))

(event `/Game/MyAssets/BPI_Weapone.Attack_Special`
  (bind _followcamera (`/Game/ThirdPerson/Blueprints/BP_ThirdPersonCharacter.FollowCamera` (`self.Ashe`)))
  (`KismetSystemLibrary.PrintString` "SPECIAL")
  (set `self.AttackSpecial_CurrentRotation` (* (/ (* (- (`self.AttackSpecial_Count`) 1) (`self.AttackSpecial_Angle`)) 2.0) -1.0))
  (for _ (range 1 (+ (`self.AttackSpecial_Count`) 1))
    (`|SpawnActorFromClass` "/Game/MyAssets/BP_Projectile_Spead.BP_Projectile_Spead_C" (`KismetMathLibrary.MakeTransform` (`SceneComponent.K2_GetComponentLocation` (`self.Muzzle`)) (`KismetMathLibrary.Conv_VectorToRotator` (`KismetMathLibrary.RotateAngleAxis` (`SceneComponent.GetForwardVector` _followcamera) (`self.AttackSpecial_CurrentRotation`) (`SceneComponent.GetUpVector` _followcamera)))) "Undefined" "MultiplyWithRoot" null null)
    (set `self.AttackSpecial_CurrentRotation` (+ (`self.AttackSpecial_CurrentRotation`) (`self.AttackSpecial_Angle`)))))

(event `/Game/MyAssets/BPI_Weapone.Attack_Ultimate`
  (`KismetSystemLibrary.PrintString` "ULTIMATE")
  (`self.ProjectUltimate`))

(event `ProjectUltimate`
  ; SPAWN DE PROYECTILES ROTACION Y DIRECCION ultimate
  (`|SpawnActorFromClass` "/Game/MyAssets/BP_Projectile_Ultimate.BP_Projectile_Ultimate_C" (`KismetMathLibrary.MakeTransform` (`SceneComponent.K2_GetComponentLocation` (`self.Muzzle`)) (`KismetMathLibrary.Conv_VectorToRotator` (`SceneComponent.GetForwardVector` (`/Game/ThirdPerson/Blueprints/BP_ThirdPersonCharacter.FollowCamera` (`self.Ashe`))))) "Undefined" "MultiplyWithRoot" null null))

(event `/Game/MyAssets/BPI_Weapone.Reload`
  (bind _ashe (`self.Ashe`))
  (bind _ashe_2 (`self.Ashe`))
  (if (and (< (`self.AmmoCurrent`) (`self.AmmoMax`)) (not (`self.IsReloading`)))
    (`/Engine/EditorBlueprintResources/StandardMacros.DoOnce` false :!label _label_5
      (:`Completed`
        (`KismetSystemLibrary.PrintString` "RECARGO")
        (set `self.IsReloading` true)
        (set `self.AmmoNeeded` (- (`self.AmmoMax`) (`self.AmmoCurrent`)))
        (if (> (`/Game/ThirdPerson/Blueprints/BP_ThirdPersonCharacter.Ammo` (`self.Ashe`)) (`self.AmmoNeeded`))
          (`KismetSystemLibrary.Delay` 1.5)
          (set `self.AmmoCurrent` (`self.AmmoMax`))
          (set `/Game/ThirdPerson/Blueprints/BP_ThirdPersonCharacter.Ammo` (- (`/Game/ThirdPerson/Blueprints/BP_ThirdPersonCharacter.Ammo` _ashe_2) (`self.AmmoNeeded`)) _ashe_2)
          (`KismetSystemLibrary.PrintString` "RELOADED FULL ")
          (elif (> (`/Game/ThirdPerson/Blueprints/BP_ThirdPersonCharacter.Ammo` (`self.Ashe`)) 0)
            (`KismetSystemLibrary.Delay` 1.5)
            (set `self.AmmoCurrent` (+ (`self.AmmoCurrent`) (`/Game/ThirdPerson/Blueprints/BP_ThirdPersonCharacter.Ammo` _ashe)))
            (set `/Game/ThirdPerson/Blueprints/BP_ThirdPersonCharacter.Ammo` 0 _ashe)
            (`KismetSystemLibrary.PrintString` "RELOADED PARCIASL ")
            (else
              (`KismetSystemLibrary.PrintString` "NOT RELOAD"))))
        (`self.ReloadColdown`)))))

(event `ReloadColdown`
  (set `self.IsReloading` false)
  (`KismetSystemLibrary.PrintString` "ACABO DE RECARGAR")
  (goto _label_5 :!via `Reset`))

(fn `UserConstructionScript`)