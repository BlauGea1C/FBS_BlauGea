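; BP_EnemyAlert is a short-lived alert actor that spreads outward and triggers a Cry reaction in the enemies it reaches.
; On BeginPlay a timeline, with play rate scaled by Duracion, grows the sphere's radius while updating overlaps, then destroys the actor when finished.
; Overlapping actors of exactly BP_Enemy or BP_Enemy_Velkoz class are cast and have Cry called on them.
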(event `self.ReceiveBeginPlay`
  (`TimelineComponent.SetPlayRate` (`self.AlertExpancion`) (/ 1.0 (`self.Duracion`)))
  (bind (_direction _alpha) (`Timeline|AlertExpancion`)
    (:`Update`
      (`SphereComponent.SetSphereRadius` (`self.Sphere`) (`KismetMathLibrary.Lerp` 32.0 2000.0 _alpha) true))
    (:`Finished`
      (`self.K2_DestroyActor`))))

(event `self.ReceiveActorBeginOverlap`
  (params (OtherActor :type "Actor Object Reference"))
  (bind _returnvalue (`GameplayStatics.GetObjectClass` OtherActor))
  (if (or (== _returnvalue "/Game/MyAssets/BP_Enemy.BP_Enemy_C") (== _returnvalue "/Game/MyAssets/BP_Enemy_Velkoz.BP_Enemy_Velkoz_C"))
    (bind _asbp_enemy_velkoz (cast `/Game/MyAssets/BP_Enemy_Velkoz` OtherActor)
      (:`then`
        (`/Game/MyAssets/BP_Enemy_Velkoz.Cry` _asbp_enemy_velkoz))
      (:`CastFailed`
        (bind _asbp_enemy (cast `/Game/MyAssets/BP_Enemy` OtherActor))
        (`/Game/MyAssets/BP_Enemy.Cry` _asbp_enemy)))))

(fn `UserConstructionScript`)