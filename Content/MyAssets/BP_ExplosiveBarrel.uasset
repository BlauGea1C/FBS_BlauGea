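; Explosive barrel actor that takes shot damage and explodes when its health reaches zero.
; OnShot feeds HealthM, which adds the signed amount to clamped health and reports depletion.
; Depletion enables the initially non-colliding Sphere, removes the barrel mesh, plays Niagara and sound effects, then destroys the actor after a short delay.
; Actors overlapping the blast sphere receive fixed damage through BPI_Damageable.
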(event `self.ReceiveBeginPlay`
  (`PrimitiveComponent.SetCollisionEnabled` (`self.Sphere`) "NoCollision"))

(event `/Game/MyAssets/BPI_Shootable.OnShot`
  (params (DirectionShoot :type "Vector Structure") (Damage :type "Float (double-precision)"))
  (`self.HealthM` Damage
    (:`true`
      (`KismetSystemLibrary.PrintString` "BOOOOOOM")
      (`PrimitiveComponent.SetCollisionEnabled` (`self.Sphere`) "QueryAndPhysics")
      (`ActorComponent.K2_DestroyComponent` (`self.Barrel`))
      (`ActorComponent.Activate` (`self.NS_BarrelExplosion`) false)
      (`GameplayStatics.PlaySound2D` "/Game/MyAssets/Sound/SC_Boom.SC_Boom" 1.0 1.0 0.0 null null)
      (`KismetSystemLibrary.Delay` 0.8)
      (`self.K2_DestroyActor`))))

(event `self.Sphere.OnComponentBeginOverlap`
  (params (OverlappedComponent :type "PrimitiveComponent Object Reference") (OtherActor :type "Actor Object Reference") (OtherComp :type "PrimitiveComponent Object Reference") (OtherBodyIndex :type Integer) (bFromSweep :type Boolean) (SweepResult :type "HitResult Structure (by ref)"))
  (if (`KismetSystemLibrary.DoesImplementInterface` OtherActor "/Game/MyAssets/BPI_Damageable.BPI_Damageable_C")
    (message `/Game/MyAssets/BPI_Damageable.OnDamaged` OtherActor -60.0)))

(fn `UserConstructionScript`)