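; BP_Projectile_Flare1 is a flare projectile actor that damages shootable actors it overlaps.
; On actor overlap, it sends BPI_Shootable's OnShotMessage with the capsule's forward vector and its Damage value.
; Logic to spawn a BP_Flare_Area at an impact point and destroy the actor after a delay is disconnected, and the capsule hit and overlap events are empty.
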(event `self.ReceiveBeginPlay`)

(event `self.ReceiveActorBeginOverlap`
  (params (OtherActor :type "Actor Object Reference"))
  (if (`KismetSystemLibrary.DoesImplementInterface` OtherActor "/Game/MyAssets/BPI_Shootable.BPI_Shootable_C")
    (message `/Game/MyAssets/BPI_Shootable.OnShot` OtherActor (`SceneComponent.GetForwardVector` (`self.Capsule`)) (`self.Damage`))))

(event `self.Capsule.OnComponentBeginOverlap`
  (params (OverlappedComponent :type "PrimitiveComponent Object Reference") (OtherActor :type "Actor Object Reference") (OtherComp :type "PrimitiveComponent Object Reference") (OtherBodyIndex :type Integer) (bFromSweep :type Boolean) (SweepResult :type "HitResult Structure (by ref)")))

(event `self.Capsule.OnComponentHit`
  (params (HitComponent :type "PrimitiveComponent Object Reference") (OtherActor :type "Actor Object Reference") (OtherComp :type "PrimitiveComponent Object Reference") (NormalImpulse :type "Vector Structure") (Hit :type "HitResult Structure (by ref)")))

(fn `UserConstructionScript`)