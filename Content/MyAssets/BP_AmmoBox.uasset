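; BP_AmmoBox is an interactable ammo pickup that adds a fixed amount of ammo to Ashe when used.
; On interact, it runs the parent logic, increases Ashe's Ammo variable and then destroys itself.
; BeginPlay, overlap and construction only call the parent, and this graph does not set the Ashe reference.
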(event `self.ReceiveBeginPlay`
  (`parent.ReceiveBeginPlay`))

(event `self.ReceiveActorBeginOverlap`
  (params (OtherActor :type "Actor Object Reference"))
  (`parent.ReceiveActorBeginOverlap` OtherActor))

(event `/Game/MyAssets/BPI_Interactable.OnInteract`
  (bind _ashe (`self.Ashe`))
  (`parent.OnInteract`)
  (set `/Game/ThirdPerson/Blueprints/BP_ThirdPersonCharacter.Ammo` (+ (`/Game/ThirdPerson/Blueprints/BP_ThirdPersonCharacter.Ammo` _ashe) 25) _ashe)
  (`self.K2_DestroyActor`))

(fn `UserConstructionScript`
  (`parent.UserConstructionScript`))