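; Sliding double door that stays locked until the player has a high enough access level.
; At BeginPlay it caches the player character and tints both panels through a shared dynamic material, colored by BPCDoorAccessControl for the required level.
; Interacting unlocks it with a green frame light and opens it, or plays a denied sound.
; Once unlocked, character overlaps drive the Door_R timeline forward and back to slide both panels with sounds.
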(event `self.ReceiveBeginPlay`
  (bind _asbp_third_person_character (cast `/Game/ThirdPerson/Blueprints/BP_ThirdPersonCharacter` (`GameplayStatics.GetPlayerCharacter` 0)))
  (set `self.Ashe` _asbp_third_person_character)
  (bind _color (`/Game/MyAssets/BPC_DoorAccessControl.GetColorDependingOnAccessLevel` (`self.BPC_DoorAccessControl`) (`self.AccessLevelRequired`)))
  (bind _returnvalue (`PrimitiveComponent.CreateDynamicMaterialInstance` (`self.SM_Door_Panel_L`) 0 "/Game/MyAssets/Door/M_DoorPanel.M_DoorPanel" "None"))
  (`MaterialInstanceDynamic.SetVectorParameterValue` _returnvalue "Color" _color)
  (`PrimitiveComponent.SetMaterial` (`self.SM_Door_Panel_R`) 0 _returnvalue))

(event `/Game/MyAssets/BPI_Interactable.OnInteract`
  (bind _returnvalue (`self.K2_GetActorLocation`))
  (if (`self.Locked`)
    (if (>= (`/Game/ThirdPerson/Blueprints/BP_ThirdPersonCharacter.AccessLevel` (`self.Ashe`)) (`self.AccessLevelRequired`))
      (`GameplayStatics.PlaySoundAtLocation` "/Game/MyAssets/Sound/SC_Door_Granted.SC_Door_Granted" _returnvalue (struct) 1.0 1.0 0.0 null null null null)
      (`KismetSystemLibrary.PrintString` "Hello")
      (set `self.Locked` false)
      (bind _returnvalue_2 (`PrimitiveComponent.CreateDynamicMaterialInstance` (`self.SM_Door_Frame`) 1 "/Game/MyAssets/Door/M_DoorLight.M_DoorLight" "None"))
      (`MaterialInstanceDynamic.SetVectorParameterValue` _returnvalue_2 "Color" (struct :`G` 1.0 :`A` 1.0))
      (`GameplayStatics.PlaySoundAtLocation` "/Game/MyAssets/Sound/SC_Door_Open.SC_Door_Open" (`self.K2_GetActorLocation`) (struct) 1.0 1.0 0.0 null null null null :!label _label)
      (bind (_direction _alpha) (`Timeline|Door_R` :!label _label_2)
        (:`Update`
          (`SceneComponent.K2_SetRelativeLocation` (`self.SM_Door_Panel_R`) (`KismetMathLibrary.VLerp` (0.0 0.0 0.0) (111.0 0.0 0.0) _alpha) false false)
          (`SceneComponent.K2_SetRelativeLocation` (`self.SM_Door_Panel_L`) (`KismetMathLibrary.VLerp` (0.0 0.0 0.0) (-80.0 0.0 0.0) _alpha) false false)))
      (else
        (`GameplayStatics.PlaySoundAtLocation` "/Game/MyAssets/Sound/SC_Door_Deneid.SC_Door_Deneid" _returnvalue (struct) 1.0 1.0 0.0 null null null null)))))

(event `self.ReceiveActorBeginOverlap`
  (params (OtherActor :type "Actor Object Reference"))
  (bind _ascharacter (cast `Character` OtherActor))
  (`/Engine/EditorBlueprintResources/StandardMacros.IsValid` _ascharacter
    (:`Is Valid`
      (if (not (`self.Locked`))
        (goto _label)))))

(event `self.ReceiveActorEndOverlap`
  (params (OtherActor :type "Actor Object Reference"))
  (bind _ascharacter (cast `Character` OtherActor))
  (`/Engine/EditorBlueprintResources/StandardMacros.IsValid` _ascharacter
    (:`Is Valid`
      (if (not (`self.Locked`))
        (`GameplayStatics.PlaySoundAtLocation` "/Game/MyAssets/Sound/SC_Door_Close.SC_Door_Close" (`self.K2_GetActorLocation`) (struct) 1.0 1.0 0.0 null null null null)
        (goto _label_2 :!via `Reverse`)))))

(fn `UserConstructionScript`)