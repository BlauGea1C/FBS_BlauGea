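; BP_IDCard is an interactable ID card pickup that grants Ashe a door access level.
; On BeginPlay it asks BPCDoorAccessControl for the color matching its AccessLevelGrantted and applies it to the mesh through a dynamic M_IDCard material instance.
; Interacting sets Ashe's AccessLevel to the granted level, overwriting the current value, then destroys the card.
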(event `self.ReceiveBeginPlay`
  (`parent.ReceiveBeginPlay`)
  (bind _color (`/Game/MyAssets/BPC_DoorAccessControl.GetColorDependingOnAccessLevel` (`self.BPC_DoorAccessControl`) (`self.AccessLevelGrantted`)))
  (bind _returnvalue (`PrimitiveComponent.CreateDynamicMaterialInstance` (`self.Mesh`) 0 "/Game/MyAssets/IDCard/M_IDCard.M_IDCard" "None"))
  (`MaterialInstanceDynamic.SetVectorParameterValue` _returnvalue "Color" _color))

(event `/Game/MyAssets/BPI_Interactable.OnInteract`
  (`parent.OnInteract`)
  (set `/Game/ThirdPerson/Blueprints/BP_ThirdPersonCharacter.AccessLevel` (`self.AccessLevelGrantted`) (`self.Ashe`))
  (`self.K2_DestroyActor`))

(fn `UserConstructionScript`
  (`parent.UserConstructionScript`))