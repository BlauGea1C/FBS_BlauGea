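; Enemy AI character (Fiddlesticks animations) that patrols, roams, guards or chases, and fights the player character Ashe.
; Sight via PawnSensing or surviving damage raises an alert that spawns BP_EnemyAlert and starts a chase; Cry starts one without spawning.
; In range, it plays distance-based attack montages, then sphere-traces forward to damage Ashe.
; A retriggerable delay drops aggro after lost sight, and zero health triggers a death montage and destruction.
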(event `self.ReceiveBeginPlay`
  (`self.LaunchBaseBehaviour`)
  (bind _asbp_third_person_character (cast `/Game/ThirdPerson/Blueprints/BP_ThirdPersonCharacter` (`GameplayStatics.GetPlayerCharacter` 0)))
  (set `self.Ashe` _asbp_third_person_character))

(event `LaunchBaseBehaviour`
  (switch `/Game/MyAssets/Enum_EnemyStates` (`self.BaseBehaviour`)
    (:`NewEnumerator0`
      (`self.BehaviourPatrol`))
    (:`NewEnumerator1`
      (`self.BehaviourRoam`))
    (:`NewEnumerator2`
      (`self.BehaviorGuard`))
    (:`NewEnumerator3`
      (`self.BehaviorChase`))))

(event `BehaviorGuard`
  ; GUARD
  (if (not (`self.HasAggro`))
    (`|AIMoveTo` self (0.0 0.0 0.0) (`self.PatrolPoint`) 1.0
      (:`OnSuccess`
        (set `self.Guard_InitialRotation` (`self.K2_GetActorRotation`))
        (set `self.Guard_EndRotation` (`self.K2_GetActorRotation` (`self.PatrolPoint`)))
        (bind (_direction _alpha) (`Timeline|GuardRotationAnimation`)
          (:`Update`
            (`self.K2_SetActorRotation` (`KismetMathLibrary.RLerp` (`self.Guard_InitialRotation`) (`self.Guard_EndRotation`) _alpha true))))))))

(event `BehaviourPatrol`
  ;[0.002623 0.15 0.001041 0.5] PATROL
  (if (not (`self.HasAggro`))
    (`|AIMoveTo` self (0.0 0.0 0.0) (`self.PatrolPoint`) 50.0
      (:`OnSuccess`
        (`KismetSystemLibrary.Delay` (`KismetMathLibrary.RandomFloatInRange` 2.0 5.0))
        (set `self.PatrolPoint` (`/Game/MyAssets/BP_PatrolPoint.NextPatrolPoit` (`self.PatrolPoint`)))
        (`self.BehaviourPatrol`)))))

(event `BehaviourRoam`
  ;[0.02807 0.02447 0.15 0.5] ROAM
  (if (not (`self.HasAggro`))
    (bind _randomlocation (`NavigationSystemV1.K2_GetRandomLocationInNavigableRadius` (`self.K2_GetActorLocation` (`self.PatrolPoint`)) (`self.RoamRadiuS`) null null))
    (if (> (`KismetMathLibrary.Vector_Distance` _randomlocation (`self.K2_GetActorLocation`)) 200.0)
      (`|AIMoveTo` self _randomlocation null 1.0
        (:`then`
          (`KismetSystemLibrary.Delay` (`KismetMathLibrary.RandomFloatInRange` 2.0 5.0))
          (`self.BehaviourRoam`)))
      (else
        (`self.BehaviourRoam`)))))

(event `/Game/MyAssets/BPI_Shootable.OnShot`
  (params (DirectionShoot :type "Vector Structure") (Damage :type "Float (double-precision)"))
  ;[0.15 0.06616 0 0.5] Daño Muerte
  ;; DañoDisparo
  (`self.HealthManager` Damage
    (:`IsDead`
      (`self.Dead`))
    (:`IsAlive`
      (if (not (`self.HasAggro`))
        (`self.BehaviorAlert`)))))

(event `/Game/MyAssets/BPI_Damageable.OnDamaged`
  (params (NewParam :type "Float (double-precision)"))
  ;[0.15 0.06616 0 0.5] Daño Muerte
  ;; DañoBarril
  (`self.HealthManager` NewParam
    (:`IsDead`
      (`self.Dead`))
    (:`IsAlive`
      (if (not (`self.HasAggro`))
        (`self.BehaviorAlert`)))))

(event `Dead`
  ;[0.15 0.06616 0 0.5] Daño Muerte
  (`/Engine/EditorBlueprintResources/StandardMacros.DoOnce` false
    (:`Completed`
      (`CharacterMovementComponent.SetMovementMode` (`self.CharacterMovement`) "MOVE_None" 0)
      (bind _returnvalue (`self.PlayAnimMontage` (`KismetArrayLibrary.Array_Random` (`self.Anim_Death`))))
      (`KismetSystemLibrary.Delay` _returnvalue)
      (`self.K2_DestroyActor`))))

(event `BehaviorAlert`
  ;[0.15 0.001176 0.0205 0.5] DETECTAR AL JUGADOR * ATACAR
  (`/Engine/EditorBlueprintResources/StandardMacros.DoOnce` false :!label _label
    (:`Completed`
      (set `self.HasAggro` true)
      (`self.BehaviorStop`)
      (`|SpawnActorFromClass` "/Game/MyAssets/BP_EnemyAlert.BP_EnemyAlert_C" (`KismetMathLibrary.MakeTransform` (`self.K2_GetActorLocation`)) "Undefined" "MultiplyWithRoot" null null)
      (bind _returnvalue (`self.PlayAnimMontage` "/Game/MyAssets/Enemys/Enemy_Fiddlesticks/AM_Fiddlesticks_AreaAlert.AM_Fiddlesticks_AreaAlert"))
      (`KismetSystemLibrary.Delay` _returnvalue)
      (`self.BehaviorChase`))))

(event `self.PawnSensing.OnSeePawn`
  (params (Pawn :type "Pawn Object Reference"))
  ;[0.15 0.001176 0.0205 0.5] DETECTAR AL JUGADOR * ATACAR
  ;; DETECTOR
  (if (== Pawn (`self.Ashe`))
    (if (not (`self.HasAggro`))
      (`self.BehaviorAlert`)
      (else
        (`self.TryNotSeePawn`)))))

(event `ResetAlert`
  ;[0.15 0.001176 0.0205 0.5] DETECTAR AL JUGADOR * ATACAR
  (goto _label :!via `Reset`))

(event `BehaviorStop`
  ;[0.15 0.001176 0.0205 0.5] DETECTAR AL JUGADOR * ATACAR
  (`|AIMoveTo` self (0.0 0.0 0.0) self))

(event `Cry`
  ;[0.15 0.001176 0.0205 0.5] DETECTAR AL JUGADOR * ATACAR
  ;; ALARMA
  (if (not (`self.HasAggro`))
    (set `self.HasAggro` true)
    (`self.BehaviorStop`)
    (bind _returnvalue (`self.PlayAnimMontage` "/Game/MyAssets/Enemys/Enemy_Fiddlesticks/AM_Fiddlesticks_Cry_Montage.AM_Fiddlesticks_Cry_Montage"))
    (`KismetSystemLibrary.Delay` _returnvalue)
    (`self.BehaviorChase`)))

(event `BehaviorChase`
  ;[0.15 0.001176 0.0205 0.5] DETECTAR AL JUGADOR * ATACAR
  ;; PERSECUCION
  (`|AIMoveTo` self (0.0 0.0 0.0) (`self.Ashe`) (`self.AttackDistance`)
    (:`OnSuccess`
      (`self.BehaviorAttack`))))

(event `TryNotSeePawn`
  ;[0.15 0.001176 0.0205 0.5] DETECTAR AL JUGADOR * ATACAR
  (`KismetSystemLibrary.RetriggerableDelay` 5.0)
  (`self.BehaviorStop`)
  (set `self.HasAggro` false)
  (`self.ResetAlert`)
  (`KismetSystemLibrary.Delay` 2.0)
  (if (not (`self.HasAggro`))
    (`self.LaunchBaseBehaviour`)))

(event `BehaviorAttack`
  ;[0.15 0.001176 0.0205 0.5] DETECTAR AL JUGADOR * ATACAR
  ;; ATAQUE
  (`/Engine/EditorBlueprintResources/StandardMacros.DoOnce` false :!label _label_2
    (:`Completed`
      (if (<= (`KismetMathLibrary.Vector_Distance` (`self.K2_GetActorLocation`) (`self.K2_GetActorLocation` (`self.Ashe`))) 2000.0)
        (`/Engine/EditorBlueprintResources/StandardMacros.FlipFlop`
          (:`A`
            (`self.PlayAnimMontage` "/Game/MyAssets/Enemys/Enemy_Fiddlesticks/AM_Fiddlesticks_CloseAttack_01.AM_Fiddlesticks_CloseAttack_01")
            (`KismetSystemLibrary.PrintString` "ATTACK 01")
            (`KismetSystemLibrary.Delay` 0.7))
          (:`B`
            (`self.PlayAnimMontage` "/Game/MyAssets/Enemys/Enemy_Fiddlesticks/AM_Fiddlesticks_CloseAttack_01.AM_Fiddlesticks_CloseAttack_01")
            (`KismetSystemLibrary.PrintString` "ATTACK 02")
            (`KismetSystemLibrary.Delay` 0.7)))
        (else
          (`self.PlayAnimMontage` "/Game/MyAssets/Enemys/Enemy_Fiddlesticks/AM_Fiddlesticks_MidAttack.AM_Fiddlesticks_MidAttack")
          (`KismetSystemLibrary.PrintString` "ATTACK MID")
          (`KismetSystemLibrary.Delay` 0.7)))
      (`self.AttackTrail`)
      (`self.ResetAttack`)
      (`self.BehaviorChase`))))

(event `ResetAttack`
  ;[0.15 0.001176 0.0205 0.5] DETECTAR AL JUGADOR * ATACAR
  ;; ATAQUE
  (goto _label_2 :!via `Reset`))

(event `AttackTrail`
  (bind _returnvalue (`self.K2_GetActorLocation`))
  ;[0.15 0.001176 0.0205 0.5] DETECTAR AL JUGADOR * ATACAR
  ;; ATAQUE
  (bind _outhit (`KismetSystemLibrary.SphereTraceSingle` :`Start` _returnvalue :`End` (+ _returnvalue (* (`self.GetActorForwardVector`) 250.0)) :`Radius` 50.0 :`TraceChannel` "TraceTypeQuery1" :`DrawDebugType` "ForDuration"))
  (if (== (`.HitActor` (`GameplayStatics.BreakHitResult` _outhit)) (`self.Ashe`))
    (`/Game/MyAssets/BPI_Damageable.OnDamaged` (`self.Ashe`) -10.0)))

(fn `UserConstructionScript`)