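; Sliding door Blueprint for the underground base that opens when a Character enters its trigger box and closes when one leaves.
; Box overlap events filter for Characters, play an open or close sound at the actor, and play or reverse the Door_Slide timeline.
; The timeline's track sets the door mesh's relative location without sweeping.
; Any Character leaving reverses the door, with no count of others still inside.
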(event `self.Box.OnComponentBeginOverlap`
  (params (OverlappedComponent :type "PrimitiveComponent Object Reference") (OtherActor :type "Actor Object Reference") (OtherComp :type "PrimitiveComponent Object Reference") (OtherBodyIndex :type Integer) (bFromSweep :type Boolean) (SweepResult :type "HitResult Structure (by ref)"))
  (bind _ascharacter (cast `Character` OtherActor))
  (`/Engine/EditorBlueprintResources/StandardMacros.IsValid` _ascharacter
    (:`Is Valid`
      (`GameplayStatics.PlaySoundAtLocation` "/Game/MyAssets/Sound/SC_Door_Open.SC_Door_Open" (`self.K2_GetActorLocation`) (struct) 1.0 1.0 0.0 null null null null)
      (bind (_direction _newtrack_0) (`Timeline|Door_Slide` :!label _label)
        (:`Update`
          (`SceneComponent.K2_SetRelativeLocation` (`self.StaticMesh`) _newtrack_0 false false))))))

(event `self.Box.OnComponentEndOverlap`
  (params (OverlappedComponent :type "PrimitiveComponent Object Reference") (OtherActor :type "Actor Object Reference") (OtherComp :type "PrimitiveComponent Object Reference") (OtherBodyIndex :type Integer))
  (bind _ascharacter (cast `Character` OtherActor))
  (`/Engine/EditorBlueprintResources/StandardMacros.IsValid` _ascharacter
    (:`Is Valid`
      (`GameplayStatics.PlaySoundAtLocation` "/Game/MyAssets/Sound/SC_Door_Close.SC_Door_Close" (`self.K2_GetActorLocation`) (struct) 1.0 1.0 0.0 null null null null)
      (goto _label :!via `Reverse`))))

(fn `UserConstructionScript`)